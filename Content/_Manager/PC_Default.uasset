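; Default player controller that turns Enhanced Input into movement, look and movement-state changes for the possessed BP_Character.
; On BeginPlay it adds the default mapping context, caches the character and its movement component, and sets crouch speed.
; Move follows control yaw, look applies sensitivity, and run, sprint and crouch inputs call AdjustMovement.
; AdjustMovement tracks current and previous states and sets walk, run or sprint speed; the Crouch/UnCrouch logic is unconnected.
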(event Input|EnhancedActionEvents|EnhancedInputActionIA_Look
  (params (ActionValue :type Vector%202D%20Structure) (ElapsedSeconds :type Float%20%28double-precision%29) (TriggeredSeconds :type Float%20%28double-precision%29) (InputAction :type Input%20Action%20Object%20Reference :default "/Game/_Manager/Input/Actions/IA_Look.IA_Look"))
  (bind _sensitivity (Variables|Default|GetSensitivity))
  (bind _returnvalue (* ActionValue _sensitivity))
  (Class|PlayerController|AddYawInput (.x _returnvalue))
  (Class|PlayerController|AddPitchInput (.y _returnvalue)))

(event Input|EnhancedActionEvents|EnhancedInputActionIA_Move
  (params (ActionValue :type Vector%202D%20Structure) (ElapsedSeconds :type Float%20%28double-precision%29) (TriggeredSeconds :type Float%20%28double-precision%29) (InputAction :type Input%20Action%20Object%20Reference :default "/Game/_Manager/Input/Actions/IA_Move.IA_Move"))
  (Pawn|Input|AddMovementInput (Pawn|GetControlledPawn) (Math|Vector|Normalize (+ (* (.x ActionValue) (Math|Vector|GetRightVector (Math|Rotator|MakeRotator 0.0 0.0 (.yaw (Pawn|GetControlRotation :!class /Script/Engine.Controller))))) (* (.y ActionValue) (Math|Vector|GetForwardVector (Math|Rotator|MakeRotator 0.0 0.0 (.yaw (Pawn|GetControlRotation :!class /Script/Engine.Controller))))))) 1.0 false))

(event Input|EnhancedActionEvents|EnhancedInputActionIA_Run
  (params (ActionValue :type Boolean) (ElapsedSeconds :type Float%20%28double-precision%29) (TriggeredSeconds :type Float%20%28double-precision%29) (InputAction :type Input%20Action%20Object%20Reference :default "/Game/_Manager/Input/Actions/IA_Run.IA_Run"))
  (CallFunction|AdjustMovement "NewEnumerator2"))

(event Input|EnhancedActionEvents|EnhancedInputActionIA_Sprint
  (params (ActionValue :type Boolean) (ElapsedSeconds :type Float%20%28double-precision%29) (TriggeredSeconds :type Float%20%28double-precision%29) (InputAction :type Input%20Action%20Object%20Reference :default "/Game/_Manager/Input/Actions/IA_Sprint.IA_Sprint"))
  (CallFunction|AdjustMovement "NewEnumerator3"))

(event Input|EnhancedActionEvents|EnhancedInputActionIA_Crouch
  (params (ActionValue :type Boolean) (ElapsedSeconds :type Float%20%28double-precision%29) (TriggeredSeconds :type Float%20%28double-precision%29) (InputAction :type Input%20Action%20Object%20Reference :default "/Game/_Manager/Input/Actions/IA_Crouch.IA_Crouch"))
  (CallFunction|AdjustMovement "NewEnumerator4"))

(event EventBeginPlay
  (Input|AddMappingContext (PlayerController|LocalPlayerSubsystems|GetEnhancedInputLocalPlayerSubsystem) "/Game/_Manager/Input/IMC_Default.IMC_Default" 0 "(bIgnoreAllPressedKeysUntilRelease=True,bForceImmediately=False,bNotifyUserSettings=False)")
  (bind _asbp_character (Utilities|Casting|CastToBP_Character (Pawn|GetControlledPawn)))
  (Variables|Default|SetActor _asbp_character)
  (Variables|Default|SetMovement (Variables|/Script/Engine.Character|GetCharacterMovement (Variables|Default|GetActor)))
  (Variables|/Script/Engine.CharacterMovementComponent|SetMaxWalkSpeedCrouched (Variables|Default|GetMovement) (Variables|Default|GetCrouchSpeed))
  (CallFunction|AdjustMovement "NewEnumerator0"))

(fn ConstructionScript)

(fn AdjustMovement
  (params (New :type E_Movement%20Enum :default "NewEnumerator0"))
  (Variables|Default|SetLastMovement (Variables|Default|GetCurrentMovement))
  (Variables|Default|SetCurrentMovement New)
  (switch Utilities|FlowControl|Switch|SwitchonE_Movement (Variables|Default|GetCurrentMovement)
    (:NewEnumerator1
      (Variables|/Script/Engine.CharacterMovementComponent|SetMaxWalkSpeed (Variables|Default|GetMovement) (Variables|Default|GetWalkSpeed)))
    (:NewEnumerator2
      (Variables|/Script/Engine.CharacterMovementComponent|SetMaxWalkSpeed (Variables|Default|GetMovement) (Variables|Default|GetRunSpeed)))
    (:NewEnumerator3
      (Variables|/Script/Engine.CharacterMovementComponent|SetMaxWalkSpeed (Variables|Default|GetMovement) (Variables|Default|GetSprintSpeed)))))